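; Behavior tree service for the Cat enemy that finds the nearest Player-tagged pawn and writes it to a blackboard key.
; On search start, it sphere-overlaps pawns around the controlled pawn and keeps the one below the stored shortest distance, which is never reset here.
; The in-radius flag follows only the last overlapped actor and decides whether the key is set or cleared.
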(event `self.ReceiveSearchStartAI`
  (params (OwnerController :type "AIController Object Reference") (ControlledPawn :type "Pawn Object Reference"))
  (bind _returnvalue (`KismetMathLibrary.Vector_Distance` (`Actor.K2_GetActorLocation` (`self.Controlled Pawn`)) (`Actor.K2_GetActorLocation` (`self.Array Element`))))
  (bind _output_get (set `self.Controlled Pawn` ControlledPawn))
  (bind _outactors (`KismetSystemLibrary.SphereOverlapActors` (`Actor.K2_GetActorLocation` _output_get) (`self.Sphere Radius`) (`|MakeArray` "ObjectTypeQuery3" :!type "EObjectTypeQuery Enum")))
  (for _array_element _outactors
    (bind _output_get_2 (set `self.Array Element` _array_element))
    (if (`Actor.ActorHasTag` _output_get_2 "Player")
      (set `self.HasPlayerInRadius` true)
      (if (< _returnvalue (`self.ActorLocation`))
        (set `self.ActorLocation` _returnvalue)
        (set `self.Player` (`self.Array Element`)))
      (else
        (set `self.HasPlayerInRadius` false))))
  (if (`self.HasPlayerInRadius`)
    (`BTFunctionLibrary.SetBlackboardValueAsObject` (`self.KeyClosestPlayer`) (`self.Player`))
    (else
      (`BTFunctionLibrary.ClearBlackboardValue` (`self.KeyClosestPlayer`)))))